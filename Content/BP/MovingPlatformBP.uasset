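; Moving platform actor that shuttles a Platform component back and forth along the world Y axis.
; Each tick it teleports the platform by MoveSpeed scaled by delta time, with the sign set by a Flip flag.
; BeginPlay seeds Flip from the Invert option to choose the starting direction.
; Overlap of the platform with either boundary box, Box or Box1, toggles Flip and reverses travel.
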(event OnComponentBeginOverlap(Box)
  (params (OverlappedComponent :type Primitive%20Component%20Object%20Reference) (OtherActor :type Actor%20Object%20Reference) (OtherComp :type Primitive%20Component%20Object%20Reference) (OtherBodyIndex :type Integer) (bFromSweep :type Boolean) (SweepResult :type Hit%20Result%20Structure%20%28by%20ref%29))
  (if (== OtherComp (Variables|Default|GetPlatform))
    (Variables|Default|SetFlip (not (Variables|Default|GetFlip)))))

(event OnComponentBeginOverlap(Box1)
  (params (OverlappedComponent :type Primitive%20Component%20Object%20Reference) (OtherActor :type Actor%20Object%20Reference) (OtherComp :type Primitive%20Component%20Object%20Reference) (OtherBodyIndex :type Integer) (bFromSweep :type Boolean) (SweepResult :type Hit%20Result%20Structure%20%28by%20ref%29))
  (if (== OtherComp (Variables|Default|GetPlatform))
    (Variables|Default|SetFlip (not (Variables|Default|GetFlip)))))

(event EventBeginPlay
  (if (Variables|Default|GetInvert)
    (Variables|Default|SetFlip true)
    (else
      (Variables|Default|SetFlip false))))

(event Collision|EventActorBeginOverlap
  (params (OtherActor :type Actor%20Object%20Reference)))

(event EventTick
  (params (DeltaSeconds :type Float%20%28single-precision%29))
  (bind _platform (Variables|Default|GetPlatform))
  (bind _returnvalue (Transformation|GetWorldLocation _platform))
  (if (Variables|Default|GetFlip)
    (Transformation|SetWorldLocation _platform (+ _returnvalue (Math|Vector|MakeVector 0.0 (* (Variables|Default|GetMoveSpeed) DeltaSeconds) 0.0)) false true)
    (else
      (Transformation|SetWorldLocation _platform (+ _returnvalue (Math|Vector|MakeVector 0.0 (* (* (Variables|Default|GetMoveSpeed) -1.0) DeltaSeconds) 0.0)) false true))))

(fn ConstructionScript)